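; Pinball-style bumper actor that knocks a BP_Ball away when the ball overlaps it.
; Bump applies a velocity-change impulse along the direction from bumper to ball and plays an attached hit sound.
; A BumpLerp timeline then drives the mechanism's vertical offset and the point light's intensity.
; The construction script creates a dynamic material for the bumper mesh, but its emissive boost update is disconnected.
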(event Custom|Bump
  (params (Ball :type BP%20Ball%20Object%20Reference))
  (Physics|AddImpulse (Variables|/Game/Blueprints/BP_Ball.BP_Ball_C|GetBall Ball) (* (Math|Vector|GetUnitDirection(Vector) (Transformation|GetActorLocation) (Transformation|GetActorLocation Ball)) 2.5e+03) "None" true)
  (Audio|SpawnSoundAttached "/Game/Assets/Sounds/BumperHit.BumperHit" (Variables|Default|GetBumperMesh))
  (bind _bumpalpha (Timeline|BumpLerp PlayFromStart)
    (:Update
      (Transformation|SetRelativeLocation (Variables|Default|GetBumperMechanism) (Math|Vector|Lerp(Vector) "0, 0, 0" "0, 0,-70.000000" _bumpalpha) false false)
      (Rendering|Components|Light|SetIntensity (Variables|Default|GetPointLight) (Math|Float|Lerp 0.0 5e+03 _bumpalpha)))))

(event EventBeginPlay)

(event Collision|EventActorBeginOverlap
  (params (OtherActor :type Actor%20Object%20Reference))
  (bind _asbp_ball (Utilities|Casting|CastToBP_Ball OtherActor))
  (CallFunction|Bump _asbp_ball))

(event EventTick
  (params (DeltaSeconds :type Float%20%28single-precision%29)))

(fn ConstructionScript
  (bind _returnvalue (Rendering|Material|CreateDynamicMaterialInstance (Variables|Default|GetBumperMesh) 0 0 :!class /Script/Engine.PrimitiveComponent))
  (Variables|Default|SetBumperTopMID _returnvalue))